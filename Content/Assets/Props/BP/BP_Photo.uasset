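; BP_Photo is an interactable photo prop that opens a close-up view of the photo.
; Interactive toggles an ObserveHUD widget fed with W_Photo, pausing the game and showing the mouse cursor while it is open.
; OnActor and OffActor switch the TriggerInteraction material parameter on and off, creating a dynamic M_Photo instance on each call.
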(event `self.ReceiveBeginPlay`)

(event `/Game/ThirdPersonCPP/Blueprints/Interaction_Interface.Interactive`
  (if (`self.ObserveOn`)
    (`Widget.RemoveFromParent` (`self.ObserveRef`))
    (`GameplayStatics.SetGamePaused` false)
    (set `PlayerController.bShowMouseCursor` false (`GameplayStatics.GetPlayerController` 0))
    (set `self.ObserveOn` false)
    (else
      (`GameplayStatics.SetGamePaused` true)
      (set `PlayerController.bShowMouseCursor` true (`GameplayStatics.GetPlayerController` 0))
      (bind _returnvalue (`|CreateWidget` "/Game/HUD/ObserveHUD.ObserveHUD_C"))
      (bind _output_get (set `self.ObserveRef` _returnvalue))
      (set `/Game/HUD/ObserveHUD.New Image` "/Game/HUD/UI_Art/Materials/W_Photo.W_Photo" _output_get)
      (`UserWidget.AddToViewport` _output_get 0)
      (set `self.ObserveOn` true))))

(event `/Game/ThirdPersonCPP/Blueprints/Interaction_Interface.OnActor`
  (bind _returnvalue (`PrimitiveComponent.CreateDynamicMaterialInstance` (`self.StaticMesh`) 0 "/Game/Assets/Props/Materials/M_Photo.M_Photo" "None"))
  (`MaterialInstanceDynamic.SetScalarParameterValue` _returnvalue "TriggerInteraction" 1.0))

(event `/Game/ThirdPersonCPP/Blueprints/Interaction_Interface.OffActor`
  (bind _returnvalue (`PrimitiveComponent.CreateDynamicMaterialInstance` (`self.StaticMesh`) 0 "/Game/Assets/Props/Materials/M_Photo.M_Photo" "None"))
  (`MaterialInstanceDynamic.SetScalarParameterValue` _returnvalue "TriggerInteraction" 0.0))

(fn `UserConstructionScript`)