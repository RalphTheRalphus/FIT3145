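; Robot enemy Blueprint that drives its own health bar widget.
; Every Tick it casts the widget component's user widget to EnemyUI and copies in the robot's current Health.
; It also looks up the Grappling_HookCharacter with GetActorOfClass each frame and sets ShowHealth only while that player is within a fixed distance.
; The graph holds no movement, combat or damage logic, and the construction script is empty.
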(event `self.ReceiveTick`
  (params (DeltaSeconds :type "Float (single-precision)"))
  ;[1 1 1] Change Enemy Health in UI
  (bind _asenemy_ui (cast `/Game/HUD/EnemyUI` (`WidgetComponent.GetUserWidgetObject` (`self.Health widgit`))))
  (bind _output_get (set `self.As Enemy UI` _asenemy_ui))
  (set `/Game/HUD/EnemyUI.EnemyHealth` (`self.Health`) _output_get)
  ;[0.1734 0.9502 1] Display Enemy Health Bar is player is close by
  (bind _returnvalue (`GameplayStatics.GetActorOfClass` "/Script/Grappling_Hook.Grappling_HookCharacter"))
  (bind _output_get_2 (set `self.Player Character` _returnvalue))
  (set `/Game/HUD/EnemyUI.ShowHealth` (<= (`KismetMathLibrary.Vector_Distance` (`self.K2_GetActorLocation` _output_get_2) (`self.K2_GetActorLocation`)) 4000.0) (`self.As Enemy UI`)))

(fn `UserConstructionScript`)